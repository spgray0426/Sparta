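; Chat game mode that runs a number baseball (strikes and balls) guessing game, with three turns per player.
; Client messages starting with "/" spend a turn and are scored against the generated number; other messages print as chat.
; Per-user turns live in the PlayerInfo map; a win, loss or all-turns-used draw resets every player and the number.
; Each player login also regenerates the number, and all feedback uses PrintString.
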(event `GotMessageFromClient`
  (params (Msg :type String) (PlayerController :type "PlayerController Object Reference") (UserId :type String))
  (bind (_value _returnvalue) (`BlueprintMapLibrary.Map_Find` (`self.PlayerInfo`) (`self.User Id`)))
  (bind (_strikes _balls _turncount) (break `/Game/GameModes/TurnDataStruct` _value))
  (set `self.SendMsg` Msg)
  (set `self.User Id` UserId)
  (set `self.Player Controller` PlayerController)
  (if (`KismetStringLibrary.StartsWith` (`self.SendMsg`) "/")
    (if _returnvalue
      (if (> _turncount 0)
        (`BlueprintMapLibrary.Map_Add` (`self.PlayerInfo`) (`self.User Id`) (make `/Game/GameModes/TurnDataStruct` 0 0 (- _turncount 1)))
        (bind (_return _strikes_2 _balls_2) (`/Game/GameModes/BPFL_NumberBaseball.CalculateStrikeBall` (`self.Generated Number`) (`KismetStringLibrary.RightChop` (`self.SendMsg`) 1)))
        (switch `int` _return
          (:`0`
            (`KismetSystemLibrary.PrintString` (`KismetTextLibrary.Conv_TextToString` (`|FormatText` "{id} 님이 패배하셨습니다" (`self.User Id`))))
            (`self.Reset`))
          (:`1`
            (`KismetSystemLibrary.PrintString` (`KismetTextLibrary.Conv_TextToString` (`|FormatText` "{id} 님이 승리하셨습니다" (`self.User Id`))))
            (`self.Reset`))
          (:`2`
            (`KismetSystemLibrary.PrintString` (`KismetTextLibrary.Conv_TextToString` (`|FormatText` "{Strikes} S {Balls} B" _strikes_2 _balls_2)))
            (bind _return_2 (`self.HasRemainingPlayers`))
            (if (not _return_2)
              (`KismetSystemLibrary.PrintString` "무승부")
              (`self.Reset`))))
        (else
          (`KismetSystemLibrary.PrintString` "모튼 턴을 사용했습니다."))))
    (else
      (`KismetSystemLibrary.PrintString` (`self.SendMsg`) true true (struct :`R` 0.969643 :`G` 1.0 :`A` 1.0) 5.0))))

(event `OnPlayerAdded`
  (params (UserId :type String))
  (`BlueprintMapLibrary.Map_Add` (`self.PlayerInfo`) UserId (make `/Game/GameModes/TurnDataStruct` 0 0 3))
  (`KismetSystemLibrary.PrintString` (`KismetStringLibrary.Concat_StrStr` UserId "login"))
  (set `self.Generated Number` (`/Game/GameModes/BPFL_NumberBaseball.GetRandomNumbers`)))

(fn `HasRemainingPlayers`
  (returns (Return :type Boolean))
  (bind _values (`BlueprintMapLibrary.Map_Values` (`self.PlayerInfo`)))
  (for _array_element _values
    (if (> (`.TurnCount_13_2C0D25DA47978ADE0C85649F8EEBFE40` (break `/Game/GameModes/TurnDataStruct` _array_element)) 0)
      (return true)))
  (return false))

(fn `Reset`
  (set `self.Generated Number` (`/Game/GameModes/BPFL_NumberBaseball.GetRandomNumbers`))
  (bind _keys (`BlueprintMapLibrary.Map_Keys` (`self.PlayerInfo`)))
  (for _array_element _keys
    (`BlueprintMapLibrary.Map_Add` (`self.PlayerInfo`) _array_element (make `/Game/GameModes/TurnDataStruct` 0 0 3))))

(fn `UserConstructionScript`)